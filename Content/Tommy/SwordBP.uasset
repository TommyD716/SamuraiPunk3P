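; Sword weapon actor that damages actors overlapping its collision while an attack is active.
; SwordActive switches the collision to the OverlapAll profile during the animation, and SwordDeactive disables it when idle.
; Overlaps with anything but the owner apply SwordDamage through a DoOnce that resets after a half-second delay, limiting hits to one per window across all targets.
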(event OnComponentBeginOverlap(SwordCollision)
  (params (OverlappedComponent :type Primitive%20Component%20Object%20Reference) (OtherActor :type Actor%20Object%20Reference) (OtherComp :type Primitive%20Component%20Object%20Reference) (OtherBodyIndex :type Integer) (bFromSweep :type Boolean) (SweepResult :type Hit%20Result%20Structure%20%28by%20ref%29))
  ;[1 1 1] Damage Application
  (if (!= OtherActor (Components|GetOwner))
    (Utilities|FlowControl|DoOnce false :!label _label
      (:Completed
        (Game|Damage|ApplyDamage OtherActor (Variables|Default|GetSwordDamage) 0 0)
        (Utilities|FlowControl|Delay 0.5)
        (goto _label Reset)))))

(event Custom|SwordActive
  ;[1 1 1] Active While Animation Plays
  (Collision|SetCollisionProfileName (Variables|Default|GetSwordCollision) "OverlapAll" true :!class /Script/Engine.PrimitiveComponent))

(event Custom|SwordDeactive
  ;[1 1 1] Not Active when Idle
  (Collision|SetCollisionEnabled (Variables|Default|GetSwordCollision) "NoCollision"))

(fn ConstructionScript)