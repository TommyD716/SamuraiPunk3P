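; Collectible code token pickup that spins and bobs, and is collected when the player character overlaps it.
; Tick applies a constant local rotation and plays the UpDown timeline, whose track drives a local offset.
; On box overlap with ThirdPersonTommy2, it decrements ColectablesLeft on ThirdPersonGameMode, destroys itself and plays a 2D collect sound.
; The DoorProgress event has no effect.
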(event OnComponentBeginOverlap(Box)
  (params (OverlappedComponent :type Primitive%20Component%20Object%20Reference) (OtherActor :type Actor%20Object%20Reference) (OtherComp :type Primitive%20Component%20Object%20Reference) (OtherBodyIndex :type Integer) (bFromSweep :type Boolean) (SweepResult :type Hit%20Result%20Structure%20%28by%20ref%29))
  ;[1 1 1] Key press to collect
  (Utilities|Casting|CastToThirdPersonTommy2 OtherActor)
  (bind _asthird_person_game_mode (Utilities|Casting|CastToThirdPersonGameMode (Game|GetGameMode)))
  (bind _result (Math|Integer|DecrementInt (Variables|/Game/ThirdPersonBP/Blueprints/ThirdPersonGameMode.ThirdPersonGameMode_C|GetColectables%20left _asthird_person_game_mode))
    (:%20%20
      (Variables|/Game/ThirdPersonBP/Blueprints/ThirdPersonGameMode.ThirdPersonGameMode_C|SetColectables%20left _asthird_person_game_mode _result)
      (Actor|DestroyActor)
      (Audio|PlaySound2D "/Game/Audio/SoundEffects/Collect_Item_Sound_Effect_Cue.Collect_Item_Sound_Effect_Cue" 1.0 1.0 0.0 0 0))))

(event Custom|DoorProgress
  (if true
    _))

(event EventTick
  (params (DeltaSeconds :type Float%20%28single-precision%29))
  ;[1 1 1] Rotate and float
  (Transformation|AddActorLocalRotation "0,1.000000, 0" false false)
  (bind _newtrack_0 (Timeline|UpDown Play)
    (:Update
      (Transformation|AddActorLocalOffset _newtrack_0 false false))))

(fn ConstructionScript)