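; Code token collectable that spins, bobs and is picked up when something overlaps its box.
; Tick adds a yaw rotation and plays the UpDown timeline, whose track drives a local position offset.
; Overlap decrements ColectablesLeft on ThirdPersonGameMode and destroys the token, with no check on the overlapping actor or key press.
; The DoorProgress event is an empty stub.
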(event OnComponentBeginOverlap(Box)
  (params (OverlappedComponent :type Primitive%20Component%20Object%20Reference) (OtherActor :type Actor%20Object%20Reference) (OtherComp :type Primitive%20Component%20Object%20Reference) (OtherBodyIndex :type Integer) (bFromSweep :type Boolean) (SweepResult :type Hit%20Result%20Structure%20%28by%20ref%29))
  ;[1 1 1] Key press to collect
  (bind _asthird_person_game_mode (Utilities|Casting|CastToThirdPersonGameMode (Game|GetGameMode)))
  (bind _result (Math|Integer|DecrementInt (Variables|/Game/ThirdPersonBP/Blueprints/ThirdPersonGameMode.ThirdPersonGameMode_C|GetColectables%20left _asthird_person_game_mode))
    (:%20%20
      (Variables|/Game/ThirdPersonBP/Blueprints/ThirdPersonGameMode.ThirdPersonGameMode_C|SetColectables%20left _asthird_person_game_mode _result)
      (Actor|DestroyActor))))

(event Custom|DoorProgress
  (if true
    _))

(event EventTick
  (params (DeltaSeconds :type Float%20%28single-precision%29))
  ;[1 1 1] Rotate and float
  (Transformation|AddActorLocalRotation "0,1.000000, 0" false false)
  (bind _newtrack_0 (Timeline|UpDown Play)
    (:Update
      (Transformation|AddActorLocalOffset _newtrack_0 false false))))

(fn ConstructionScript)